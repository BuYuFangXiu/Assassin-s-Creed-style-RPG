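; Enemy Blueprint that can be stealth-killed from behind.
; An overlap radius shows the assassination widget while the third-person character is inside, and Tick rotates it to face the player camera.
; StealthBackAssassination plays the paired knife victim montage, triggers a delayed mesh ragdoll and hides the widget.
; It returns the AssassinREF world location and the enemy's rotation, giving the caller a transform for the paired animation.
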(event `self.ReceiveTick`
  (params (DeltaSeconds :type "Float (single-precision)"))
  (bind _assassinate_widget (`self.Assassinate Widget`))
  ; 可刺杀UI跟随人物视角的转动而转动
  (`SceneComponent.K2_SetWorldRotation` _assassinate_widget (`KismetMathLibrary.FindLookAtRotation` (`SceneComponent.K2_GetComponentLocation` _assassinate_widget) (`SceneComponent.K2_GetComponentLocation` (`PlayerCameraManager.TransformComponent` (`GameplayStatics.GetPlayerCameraManager` 0)))) false false))

(event `Rogdoll`
  ; 布娃娃效果
  (`KismetSystemLibrary.Delay` 2.5)
  (`PrimitiveComponent.SetSimulatePhysics` (`self.Mesh`) true))

(event `self. Assasination Radius.OnComponentBeginOverlap`
  (params (OverlappedComponent :type "PrimitiveComponent Object Reference") (OtherActor :type "Actor Object Reference") (OtherComp :type "PrimitiveComponent Object Reference") (OtherBodyIndex :type Integer) (bFromSweep :type Boolean) (SweepResult :type "HitResult Structure (by ref)"))
  ; 可刺杀的UI界面：接近敌人背后出现可刺杀标志
  (cast `/Game/ThirdPerson/Blueprints/BP_ThirdPersonCharacter` OtherActor)
  (`SceneComponent.SetVisibility` (`self.Assassinate Widget`) true false))

(event `self. Assasination Radius.OnComponentEndOverlap`
  (params (OverlappedComponent :type "PrimitiveComponent Object Reference") (OtherActor :type "Actor Object Reference") (OtherComp :type "PrimitiveComponent Object Reference") (OtherBodyIndex :type Integer))
  ; 可刺杀的UI界面：离开敌人背后刺杀标志消失
  (cast `/Game/ThirdPerson/Blueprints/BP_ThirdPersonCharacter` OtherActor)
  (`SceneComponent.SetVisibility` (`self.Assassinate Widget`) false false))

(fn `Stealth Back Assassination`
  (returns (`REF Location` :type "Vector Structure") (`Assassin Rotation` :type "Rotator Structure"))
  (`self.PlayAnimMontage` "/Game/RPG_Character/Animations/Assassinations/Paired_Knife_Stealth_KidneyAndNeck_Vic1_Montage.Paired_Knife_Stealth_KidneyAndNeck_Vic1_Montage")
  (`self.Rogdoll`)
  (`SceneComponent.SetVisibility` (`self.Assassinate Widget`) false false)
  (return (`SceneComponent.K2_GetComponentLocation` (`self.Assassin REF`)) (`self.K2_GetActorRotation`)))

(fn `UserConstructionScript`)