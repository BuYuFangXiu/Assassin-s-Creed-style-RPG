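; Combat component for BP_ThirdPersonCharacter that runs a four-step melee combo and bow aiming.
; Attack input plays montages by AttackIndex, buffering presses made mid-attack for SwordAttackCombo to continue or reset the chain.
; A looping-timer sphere trace between sword points and a one-shot kick trace damage "Damegeable"-tagged actors, adding blood and camera shake.
; Bow input toggles aim rotation and a crosshair widget, without firing logic here.
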(event Custom|SwordAttack
  ;[0.15 0.15 0.15 0.5] 连击系统
  ;;[0.15 0.15 0.15 0.5] 剑攻击
  (if (Variables|Default|GetIs%20Attacking?)
    (Variables|Default|SetSave%20Attack? true)
    (else
      (Variables|Default|SetIs%20Attacking? true)
      (switch int (Variables|Default|GetAttack%20Index)
        (:0
          (CallFunction|Attack1))
        (:1
          (CallFunction|Attack2))
        (:2
          (CallFunction|Attack3))
        (:3
          (CallFunction|Attack4))))))

(event Custom|Sword%20Attack%20Combo
  ;[0.15 0.15 0.15 0.5] 连击系统
  ;;[0.15 0.15 0.15 0.5] 连击
  (if (Variables|Default|GetSave%20Attack?)
    (Variables|Default|SetSave%20Attack? false)
    (switch int (Variables|Default|GetAttack%20Index)
      (:0
        (CallFunction|Attack1))
      (:1
        (CallFunction|Attack2))
      (:2
        (CallFunction|Attack3))
      (:3
        (CallFunction|Attack4)))
    (else
      (CallFunction|StopCombo))))

(event Custom|Sphere%20Trace
  (bind _character_bp (Variables|Default|GetCharacter%20BP))
  (bind _sphere_trace (Variables|/Game/RPG_Character/ThirdPerson/Blueprints/BP_ThirdPersonCharacter.BP_ThirdPersonCharacter_C|GetSphere%20Trace _character_bp))
  (bind _returnvalue (Transformation|GetWorldLocation _sphere_trace))
  ;[0.15 0.15 0.15 0.5] 通用伤害追踪（踢击以及更多其他）
  (bind (_outhit _returnvalue_2) (Collision|SphereTraceByChannel _returnvalue _returnvalue 5e+01 "TraceTypeQuery1" false 0 "None" true "(R=1.000000,G=0.000000,B=0.000000,A=1.000000)" "(R=0.000000,G=1.000000,B=0.000000,A=1.000000)" 0.2))
  (if _returnvalue_2
    (if (Actor|ActorHasTag (.HitActor (Collision|BreakHitResult _outhit)) "Damegeable")
      (Game|Damage|ApplyDamage (.HitActor (Collision|BreakHitResult _outhit)) (Variables|Default|GetKich%20Damage) 0 0)
      (Camera|PlayWorldCameraShake "/Game/BluePrints/BP_CameraShake_SwordHit.BP_CameraShake_SwordHit_C" (.Location (Collision|BreakHitResult _outhit)) 0.0 2e+03)
      (Effects|SpawnEmitteratLocation "/Game/FXs/Particles/Blood/P_Blood_Splat_Cone.P_Blood_Splat_Cone" (.Location (Collision|BreakHitResult _outhit)) (Math|Rotator|MakeRotfromXY (.Normal (Collision|BreakHitResult _outhit)) (.Normal (Collision|BreakHitResult _outhit))) "0.400000,0.400000,0.400000" true "AutoRelease"))))

(event Custom|Play%20Sword%20Hit%20Sounds
  ;[0.15 0.15 0.15 0.5] 连击系统
  ;;[0.15 0.15 0.15 0.5] 播放剑击打声音
  (Audio|PlaySoundatLocation "/Game/Audio/Sword_Hit/MS_SwordHit.MS_SwordHit" (Transformation|GetActorLocation (Components|GetOwner)) "0, 0, 0" 1.0 1.0 0.0 0 0 0 0))

(event Custom|Stop%20Combo
  ;[0.15 0.15 0.15 0.5] 连击系统
  ;;[0.15 0.15 0.15 0.5] 停止攻击和连击
  (Variables|Default|SetIs%20Attacking? false)
  (Variables|Default|SetAttack%20Index 0))

(event Custom|Attack%204
  ;[0.15 0.15 0.15 0.5] 连击系统
  ;;[0.15 0.15 0.15 0.5] 攻击4
  (Utilities|FlowControl|DoOnce false :!label _label
    (:Completed
      (Utilities|FlowControl|Delay 0.1)
      (Animation|Montage|PlayMontage (Variables|Default|GetCharacter%20Mesh) "/Game/RPG_Character/Animations/SwordAttacks/Attack3_Montage.Attack3_Montage"
        (:then
          (Variables|Default|SetAttack%20Index 0)
          (goto _label Reset))))))

(event Custom|Attack%201
  ;[0.15 0.15 0.15 0.5] 连击系统
  ;;[0.15 0.15 0.15 0.5] 攻击1
  (Utilities|FlowControl|DoOnce false :!label _label
    (:Completed
      (Utilities|FlowControl|Delay 0.1)
      (Animation|Montage|PlayMontage (Variables|Default|GetCharacter%20Mesh) "/Game/RPG_Character/Animations/SwordAttacks/Attack1_Montage.Attack1_Montage"
        (:then
          (Variables|Default|SetAttack%20Index 1)
          (goto _label Reset))))))

(event Custom|Start%20Sword%20Trace
  ;[0.15 0.15 0.15 0.5] 剑的伤害追踪
  (bind _returnvalue (Utilities|Time|SetTimerbyEvent (delegate Custom|Sword%20Trace%20Loop) 0.001 true))
  (Variables|Default|SetSwordTraceLoop _returnvalue))

(event Custom|Attack%202
  ;[0.15 0.15 0.15 0.5] 连击系统
  ;;[0.15 0.15 0.15 0.5] 攻击2
  (Utilities|FlowControl|DoOnce false :!label _label
    (:Completed
      (Utilities|FlowControl|Delay 0.1)
      (Animation|Montage|PlayMontage (Variables|Default|GetCharacter%20Mesh) "/Game/RPG_Character/Animations/SwordAttacks/Attack2_Montage.Attack2_Montage"
        (:then
          (Variables|Default|SetAttack%20Index 2)
          (goto _label Reset))))))

(event Custom|Sword%20Trace%20Loop
  ;[0.15 0.15 0.15 0.5] 剑的伤害追踪
  (bind (_outhit _returnvalue) (Collision|SphereTraceByChannel (Transformation|GetWorldLocation (Variables|/Game/RPG_Character/ThirdPerson/Blueprints/BP_ThirdPersonCharacter.BP_ThirdPersonCharacter_C|GetSword%20Top%20Point (Variables|Default|GetCharacter%20BP))) (Transformation|GetWorldLocation (Variables|/Game/RPG_Character/ThirdPerson/Blueprints/BP_ThirdPersonCharacter.BP_ThirdPersonCharacter_C|GetSword%20Bottom%20Point (Variables|Default|GetCharacter%20BP))) 1e+01 "TraceTypeQuery1" false 0 "None" true "(R=1.000000,G=0.000000,B=0.000000,A=1.000000)" "(R=0.000000,G=1.000000,B=0.000000,A=1.000000)" 0.2))
  (if _returnvalue
    (if (Actor|ActorHasTag (.HitActor (Collision|BreakHitResult _outhit)) "Damegeable")
      (Utilities|FlowControl|DoOnce false :!label _label
        (:Completed
          (Game|Damage|ApplyDamage (.HitActor (Collision|BreakHitResult _outhit)) (Variables|Default|GetSword%20Damage) 0 0)
          (Camera|PlayWorldCameraShake "/Game/BluePrints/BP_CameraShake_SwordHit.BP_CameraShake_SwordHit_C" (.Location (Collision|BreakHitResult _outhit)) 0.0 2e+03)
          (CallFunction|PlaySwordHitSounds)
          (Effects|SpawnEmitteratLocation "/Game/FXs/Particles/Blood/P_Blood_Splat_Cone.P_Blood_Splat_Cone" (.Location (Collision|BreakHitResult _outhit)) (Math|Rotator|MakeRotfromXY (.Normal (Collision|BreakHitResult _outhit)) (.Normal (Collision|BreakHitResult _outhit))) "0.400000,0.400000,0.400000" true "AutoRelease")
          (Utilities|FlowControl|Delay 0.3)
          (goto _label Reset))))))

(event Custom|Attack%203
  ;[0.15 0.15 0.15 0.5] 连击系统
  ;;[0.15 0.15 0.15 0.5] 攻击3
  (Utilities|FlowControl|DoOnce false :!label _label
    (:Completed
      (Utilities|FlowControl|Delay 0.1)
      (Animation|Montage|PlayMontage (Variables|Default|GetCharacter%20Mesh) "/Game/RPG_Character/Animations/SwordAttacks/Kick_Montage.Kick_Montage"
        (:then
          (Variables|Default|SetAttack%20Index 3)
          (goto _label Reset))))))

(event Custom|Stop%20Sword%20Trace
  ;[0.15 0.15 0.15 0.5] 剑的伤害追踪
  ;;[0.15 0.15 0.15 0.5] 中断攻击连击
  (Utilities|Time|ClearandInvalidateTimerbyHandle (Variables|Default|GetSwordTraceLoop)))

(event Input|EnhancedActionEvents|EnhancedInputActionIA_Attack
  (params (ActionValue :type Boolean) (ElapsedSeconds :type Float%20%28double-precision%29) (TriggeredSeconds :type Float%20%28double-precision%29) (InputAction :type Input%20Action%20Object%20Reference :default "/Game/Input/Actions/IA_Attack.IA_Attack"))
  ;[0.15 0.15 0.15 0.5] 连击系统
  ;;[0.15 0.15 0.15 0.5] 攻击输入
  (:Started
    (if (Variables|Default|GetCan%20Attack?)
      (CallFunction|SwordAttack))))

(event Input|EnhancedActionEvents|EnhancedInputActionIA_BowShoot
  (params (ActionValue :type Boolean) (ElapsedSeconds :type Float%20%28double-precision%29) (TriggeredSeconds :type Float%20%28double-precision%29) (InputAction :type Input%20Action%20Object%20Reference :default "/Game/Input/Actions/IA_BowShoot.IA_BowShoot"))
  (bind _character_bp (Variables|Default|GetCharacter%20BP))
  (bind _character_bp_2 (Variables|Default|GetCharacter%20BP))
  (bind _charactermovement (Variables|/Script/Engine.Character|GetCharacterMovement _character_bp))
  (bind _charactermovement_2 (Variables|/Script/Engine.Character|GetCharacterMovement _character_bp_2))
  ;[0.15 0.15 0.15 0.5] 拉弓/射箭
  (:Started
    (if (Variables|Default|GetHas%20Bow?)
      (Variables|Default|SetCan%20Attack? false)
      (Variables|Default|SetAiming%20Bow true)
      (Default|EquipBowinHands _character_bp_2)
      (Variables|/Script/Engine.CharacterMovementComponent|SetbUseControllerDesiredRotation _charactermovement_2 true)
      (Variables|/Script/Engine.CharacterMovementComponent|SetbOrientRotationToMovement _charactermovement_2 false)
      (bind _returnvalue (UserInterface|CreateWidget "/Game/RPG_Character/UI/WB_Bow_Crosshair.WB_Bow_Crosshair_C"))
      (bind _output_get (Variables|Default|SetBow%20Crosshair%20Widget _returnvalue))
      (UserInterface|Viewport|AddtoViewport _output_get 0)))
  (:Completed
    (if (Variables|Default|GetHas%20Bow?)
      (Variables|Default|SetCan%20Attack? false)
      (Variables|Default|SetAiming%20Bow false)
      (Default|EquipBowinHands _character_bp)
      (Variables|/Script/Engine.CharacterMovementComponent|SetbUseControllerDesiredRotation _charactermovement false)
      (Variables|/Script/Engine.CharacterMovementComponent|SetbOrientRotationToMovement _charactermovement true)
      (Utilities|FlowControl|Delay 0.2)
      (bind _bow_crosshair_widget (Variables|Default|GetBow%20Crosshair%20Widget)
        (:then
          (Widget|RemovefromParent _bow_crosshair_widget)
          (Variables|Default|SetBow%20Crosshair%20Widget 0))
        (:else)))))

(event EventBeginPlay
  ;[0.15 0.15 0.15 0.5] 连击系统
  ;;[0.15 0.15 0.15 0.5] 初始化
  (bind _asbp_third_person_character (Utilities|Casting|CastToBP_ThirdPersonCharacter (Components|GetOwner)))
  (Variables|Default|SetCharacter%20BP _asbp_third_person_character)
  (Variables|Default|SetCharacter%20Mesh (Variables|/Script/Engine.Character|GetMesh _asbp_third_person_character)))

(event Input|KeyboardEvents|DebugKeyQ
  (params (Key :type Key%20Structure :default "None") (ActionValue :type Input%20Action%20Value%20Structure))
  ;[0.15 0.15 0.15 0.5] 收弓
  (:Pressed
    (if (Variables|Default|GetHas%20Bow?)
      (Default|UnequipBowinHands (Variables|Default|GetCharacter%20BP)))))