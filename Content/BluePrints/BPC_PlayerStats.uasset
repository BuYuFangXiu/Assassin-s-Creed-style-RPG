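; Actor component holding health, stamina, XP and level for the player, enemy and AI characters.
; On BeginPlay it waits a tick, casts its owner to set the character type, then fills that character's HUD widget.
; DecreaseHealth updates the matching HUD and, like DecreaseStamina, returns true on depletion.
; Other stat functions write only to the player HUD; enough XP triggers a level-up that resets XP, raises MaxXP and plays sounds.
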(event `self.ReceiveBeginPlay`
  (`KismetSystemLibrary.DelayUntilNextTick`)
  (bind _asbp_third_person_character (cast `/Game/RPG_Character/ThirdPerson/Blueprints/BP_ThirdPersonCharacter` (`self.GetOwner`))
    (:`then`
      (set `self.Player Character BP` _asbp_third_person_character)
      (set `self.IsPlayer` true)
      (set `self.Character Type Index` "NewEnumerator0")
      (`ProgressBar.SetPercent` (`/Game/RPG_Character/UI/WB_PlayerHUD.StaminaBar` (`/Game/RPG_Character/ThirdPerson/Blueprints/BP_ThirdPersonCharacter.HUD Widget` (`self.Player Character BP`))) (/ (`self.Current Stamina`) (`self.Max Stamina`))))
    (:`CastFailed`
      (bind _asbp_enemy (cast `/Game/BluePrints/BP_Enemy` (`self.GetOwner`))
        (:`then`
          (set `self.Enemy BP` _asbp_enemy)
          (set `self.IsPlayer` false)
          (set `self.Character Type Index` "NewEnumerator1"))
        (:`CastFailed`
          (bind _asbp_ai (cast `/Game/AI/BP_AI` (`self.GetOwner`)))
          (set `self.AI BP` _asbp_ai)
          (set `self.IsPlayer` false)
          (set `self.Character Type Index` "NewEnumerator2")))))
  (`ProgressBar.SetPercent` (select `/Game/BluePrints/E_CharacterTypes` (`self.Character Type Index`) :`NewEnumerator0` (`/Game/RPG_Character/UI/WB_PlayerHUD.HealthBar` (`/Game/RPG_Character/ThirdPerson/Blueprints/BP_ThirdPersonCharacter.HUD Widget` (`self.Player Character BP`))) :`NewEnumerator1` (`/Game/RPG_Character/UI/WB_EnemyHUD.HealthBar` (`/Game/BluePrints/BP_Enemy.HUD Widget` (`self.Enemy BP`))) :`NewEnumerator2` (`/Game/RPG_Character/UI/WB_EnemyHUD.HealthBar` (`/Game/AI/BP_AI.HUD Widget` (`self.AI BP`)))) (/ (`self.Current Health`) (`self.Max Health`)))
  (`TextBlock.SetText` (select `/Game/BluePrints/E_CharacterTypes` (`self.Character Type Index`) :`NewEnumerator0` (`/Game/RPG_Character/UI/WB_PlayerHUD.HealthText` (`/Game/RPG_Character/ThirdPerson/Blueprints/BP_ThirdPersonCharacter.HUD Widget` (`self.Player Character BP`))) :`NewEnumerator1` (`/Game/RPG_Character/UI/WB_EnemyHUD.HealthText` (`/Game/BluePrints/BP_Enemy.HUD Widget` (`self.Enemy BP`))) :`NewEnumerator2` (`/Game/RPG_Character/UI/WB_EnemyHUD.HealthText` (`/Game/AI/BP_AI.HUD Widget` (`self.AI BP`)))) (`KismetTextLibrary.Conv_DoubleToText` (`self.Current Health`) "HalfToEven"))
  (if (`self.IsPlayer`)
    (`ProgressBar.SetPercent` (`/Game/RPG_Character/UI/WB_PlayerHUD.XPBar` (`/Game/RPG_Character/ThirdPerson/Blueprints/BP_ThirdPersonCharacter.HUD Widget` (`self.Player Character BP`))) (/ (`self.XP`) (`self.Max XP`)))
    (`TextBlock.SetText` (`/Game/RPG_Character/UI/WB_PlayerHUD.XPText` (`/Game/RPG_Character/ThirdPerson/Blueprints/BP_ThirdPersonCharacter.HUD Widget` (`self.Player Character BP`))) (`|FormatText` "{Current XP} / {Max XP}" (`self.XP`) (`self.Max XP`)))
    (`TextBlock.SetText` (`/Game/RPG_Character/UI/WB_PlayerHUD.LevelText` (`/Game/RPG_Character/ThirdPerson/Blueprints/BP_ThirdPersonCharacter.HUD Widget` (`self.Player Character BP`))) (`KismetTextLibrary.Conv_IntToText` (`self.Level`)))))

(fn `Decrease Health`
  (params (Damage :type "Float (double-precision)"))
  (returns (`Is Player Death?` :type Boolean))
  (if (> (`self.Current Health`) 0.0)
    (bind _output_get (set `self.Current Health` (- (`self.Current Health`) Damage)))
    (`ProgressBar.SetPercent` (select `/Game/BluePrints/E_CharacterTypes` (`self.Character Type Index`) :`NewEnumerator0` (`/Game/RPG_Character/UI/WB_PlayerHUD.HealthBar` (`/Game/RPG_Character/ThirdPerson/Blueprints/BP_ThirdPersonCharacter.HUD Widget` (`self.Player Character BP`))) :`NewEnumerator1` (`/Game/RPG_Character/UI/WB_EnemyHUD.HealthBar` (`/Game/BluePrints/BP_Enemy.HUD Widget` (`self.Enemy BP`))) :`NewEnumerator2` (`/Game/RPG_Character/UI/WB_EnemyHUD.HealthBar` (`/Game/AI/BP_AI.HUD Widget` (`self.AI BP`)))) (/ _output_get (`self.Max Health`)))
    (`TextBlock.SetText` (select `/Game/BluePrints/E_CharacterTypes` (`self.Character Type Index`) :`NewEnumerator0` (`/Game/RPG_Character/UI/WB_PlayerHUD.HealthText` (`/Game/RPG_Character/ThirdPerson/Blueprints/BP_ThirdPersonCharacter.HUD Widget` (`self.Player Character BP`))) :`NewEnumerator1` (`/Game/RPG_Character/UI/WB_EnemyHUD.HealthText` (`/Game/BluePrints/BP_Enemy.HUD Widget` (`self.Enemy BP`))) :`NewEnumerator2` (`/Game/RPG_Character/UI/WB_EnemyHUD.HealthText` (`/Game/AI/BP_AI.HUD Widget` (`self.AI BP`)))) (`KismetTextLibrary.Conv_DoubleToText` (`self.Current Health`) "HalfToEven"))
    (if (<= (`self.Current Health`) 0.0)
      _
      (else
        (return false))))
  (return true))

(fn `Decrease Stamina`
  (params (`Stamina Cost` :type "Float (double-precision)"))
  (returns (`No Stamina Left` :type Boolean))
  (if (> (`self.Current Stamina`) 0.0)
    (set `self.Current Stamina` (- (`self.Current Stamina`) `Stamina Cost`))
    (`ProgressBar.SetPercent` (`/Game/RPG_Character/UI/WB_PlayerHUD.StaminaBar` (`/Game/RPG_Character/ThirdPerson/Blueprints/BP_ThirdPersonCharacter.HUD Widget` (`self.Player Character BP`))) (/ (`self.Current Stamina`) (`self.Max Stamina`)))
    (if (<= (`self.Current Stamina`) 0.0)
      _
      (else
        (return false))))
  (return true))

(fn `Increase Health`
  (params (`Health Increase` :type "Float (double-precision)"))
  (bind _current_health (`self.Current Health`))
  (bind _hud_widget (`/Game/RPG_Character/ThirdPerson/Blueprints/BP_ThirdPersonCharacter.HUD Widget` (`self.Player Character BP`)))
  (set `self.Current Health` (+ (`self.Current Health`) `Health Increase`))
  (if (> (`self.Current Health`) (`self.Max Health`))
    (set `self.Current Stamina` (`self.Max Health`)))
  (`ProgressBar.SetPercent` (`/Game/RPG_Character/UI/WB_PlayerHUD.HealthBar` _hud_widget) (/ _current_health (`self.Max Health`)))
  (`TextBlock.SetText` (`/Game/RPG_Character/UI/WB_PlayerHUD.HealthText` _hud_widget) (`KismetTextLibrary.Conv_DoubleToText` _current_health "HalfToEven")))

(fn `Increase Level`
  (params (`Added Level` :type Integer))
  (set `self.Level` (+ (`self.Level`) `Added Level`))
  (set `self.Max XP` (+ (`self.Max XP`) 100.0))
  (set `self.XP` 0.0)
  (`TextBlock.SetText` (`/Game/RPG_Character/UI/WB_PlayerHUD.LevelText` (`/Game/RPG_Character/ThirdPerson/Blueprints/BP_ThirdPersonCharacter.HUD Widget` (`self.Player Character BP`))) (`KismetTextLibrary.Conv_IntToText` (`self.Level`)))
  (`GameplayStatics.PlaySound2D` "/Game/Audio/UI/LevelUp1.LevelUp1" 1.0 1.0 0.0 null null)
  (`GameplayStatics.PlaySound2D` "/Game/Audio/UI/LevelUp2.LevelUp2" 1.0 1.0 0.0 null null))

(fn `Increase Max Health`
  (params (`Max Health Increase` :type "Float (double-precision)"))
  (bind _hud_widget (`/Game/RPG_Character/ThirdPerson/Blueprints/BP_ThirdPersonCharacter.HUD Widget` (`self.Player Character BP`)))
  (set `self.Max Health` (+ (`self.Max Health`) `Max Health Increase`))
  (`ProgressBar.SetPercent` (`/Game/RPG_Character/UI/WB_PlayerHUD.HealthBar` _hud_widget) (/ (`self.Current Health`) (`self.Max Health`)))
  (`TextBlock.SetText` (`/Game/RPG_Character/UI/WB_PlayerHUD.HealthText` _hud_widget) (`KismetTextLibrary.Conv_DoubleToText` (`self.Current Health`) "HalfToEven")))

(fn `Increase Max Stamina`
  (params (`Max Stamina Regen` :type "Float (double-precision)"))
  (set `self.Max Stamina` (+ (`self.Max Stamina`) `Max Stamina Regen`))
  (`ProgressBar.SetPercent` (`/Game/RPG_Character/UI/WB_PlayerHUD.StaminaBar` (`/Game/RPG_Character/ThirdPerson/Blueprints/BP_ThirdPersonCharacter.HUD Widget` (`self.Player Character BP`))) (/ (`self.Current Stamina`) (`self.Max Stamina`))))

(fn `Increase Stamina`
  (params (`Stamina Regen` :type "Float (double-precision)"))
  (set `self.Current Stamina` (+ (`self.Current Stamina`) `Stamina Regen`))
  (if (> (`self.Current Stamina`) (`self.Max Stamina`))
    (set `self.Max Stamina` (`self.Current Stamina`)))
  (`ProgressBar.SetPercent` (`/Game/RPG_Character/UI/WB_PlayerHUD.StaminaBar` (`/Game/RPG_Character/ThirdPerson/Blueprints/BP_ThirdPersonCharacter.HUD Widget` (`self.Player Character BP`))) (/ (`self.Current Stamina`) (`self.Max Stamina`))))

(fn `Increase XP`
  (params (`Added XP` :type "Float (double-precision)"))
  (set `self.XP` (+ (`self.XP`) `Added XP`))
  (if (>= (`self.XP`) (`self.Max XP`))
    (`self.Increase Level` 1))
  (`ProgressBar.SetPercent` (`/Game/RPG_Character/UI/WB_PlayerHUD.XPBar` (`/Game/RPG_Character/ThirdPerson/Blueprints/BP_ThirdPersonCharacter.HUD Widget` (`self.Player Character BP`))) (/ (`self.XP`) (`self.Max XP`)))
  (`TextBlock.SetText` (`/Game/RPG_Character/UI/WB_PlayerHUD.XPText` (`/Game/RPG_Character/ThirdPerson/Blueprints/BP_ThirdPersonCharacter.HUD Widget` (`self.Player Character BP`))) (`|FormatText` "{Current XP} / {Max XP}" (`self.XP`) (`self.Max XP`))))