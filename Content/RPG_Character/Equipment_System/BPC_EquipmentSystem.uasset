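; Equipment component for the third-person character that handles weapon pickup and the equipment menu.
; On interact, a sphere trace from the follow camera finds a BP_Weapon, stores its item data in WeaponSlots and destroys the actor.
; The menu input toggles a lazily created, reused WB_Equipment widget, switching cursor and input mode while disabling attacks through BPCAttackSystem and halting movement.
; A debug key prints the stored weapon row names.
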(event Input|EnhancedActionEvents|EnhancedInputActionIA_Interact
  (params (ActionValue :type Boolean) (ElapsedSeconds :type Float%20%28double-precision%29) (TriggeredSeconds :type Float%20%28double-precision%29) (InputAction :type Input%20Action%20Object%20Reference :default "/Game/Input/Actions/IA_Interact.IA_Interact"))
  (bind _follow_camera (Variables|Default|GetFollow%20Camera))
  (bind _returnvalue (Transformation|GetWorldLocation _follow_camera))
  ;[0.15 0.15 0.15 0.5] 拾取武器（利用球形追踪）
  (:Started
    (bind (_outhit _returnvalue_2) (Collision|SphereTraceForObjects _returnvalue (+ _returnvalue (* (Math|Vector|GetForwardVector (Transformation|GetWorldRotation _follow_camera)) 5e+02)) 5e+01 (Utilities|Array|MakeArray "ObjectTypeQuery2") false 0 "ForDuration"))
    (if _returnvalue_2
      (bind _asbp_weapon (Utilities|Casting|CastToBP_Weapon (.HitActor (Collision|BreakHitResult _outhit))))
      (CallFunction|AddWeapon (Variables|/Game/RPG_Character/Equipment_System/BP_Weapon.BP_Weapon_C|GetItemData _asbp_weapon))
      (Actor|DestroyActor _asbp_weapon)
      (Development|PrintString "Pick Up Weapon !"))))

(event Input|EnhancedActionEvents|EnhancedInputActionIA_EquipmentMenu
  (params (ActionValue :type Boolean) (ElapsedSeconds :type Float%20%28double-precision%29) (TriggeredSeconds :type Float%20%28double-precision%29) (InputAction :type Input%20Action%20Object%20Reference :default "/Game/Input/Actions/IA_EquipmentMenu.IA_EquipmentMenu"))
  (bind _returnvalue (Game|GetPlayerController 0))
  (bind _returnvalue_2 (Components|GetOwner))
  ;[0.15 0.15 0.15 0.5] 装备菜单面板
  (:Started
    (if (not (Variables|Default|GetIsPanelOpened?))
      (bind _equipment_widge (Variables|Default|GetEquipment%20Widge)
        (:then
          (Widget|SetVisibility _equipment_widge "Visible"))
        (:else
          (bind _returnvalue_3 (UserInterface|CreateWidget "/Game/RPG_Character/Equipment_System/UI/WB_Equipment.WB_Equipment_C"))
          (bind _output_get (Variables|Default|SetEquipment%20Widge _returnvalue_3))
          (UserInterface|Viewport|AddtoViewport _output_get 0)))
      (Variables|/Game/BluePrints/BPC_AttackSystem.BPC_AttackSystem_C|SetCan%20Attack? (Variables|Default|GetBPC%20Attack%20System) false)
      (Variables|Default|SetIsPanelOpened? true)
      (Variables|/Script/Engine.PlayerController|SetbShowMouseCursor _returnvalue true)
      (Input|SetInputModeGameandUI _returnvalue (Variables|Default|GetEquipment%20Widge) "DoNotLock" true false)
      (bind _asbp_third_person_character (Utilities|Casting|CastToBP_ThirdPersonCharacter _returnvalue_2))
      (Pawn|Components|CharacterMovement|SetMovementMode (Variables|/Script/Engine.Character|GetCharacterMovement _asbp_third_person_character) "MOVE_None" 0)
      (else
        (bind _equipment_widge_2 (Variables|Default|GetEquipment%20Widge)
          (:then
            (Widget|SetVisibility _equipment_widge_2 "Hidden")
            (Variables|/Game/BluePrints/BPC_AttackSystem.BPC_AttackSystem_C|SetCan%20Attack? (Variables|Default|GetBPC%20Attack%20System) true)
            (Variables|Default|SetIsPanelOpened? false)
            (Variables|/Script/Engine.PlayerController|SetbShowMouseCursor _returnvalue false)
            (Input|SetInputModeGameOnly _returnvalue false)
            (bind _asbp_third_person_character_2 (Utilities|Casting|CastToBP_ThirdPersonCharacter _returnvalue_2))
            (Pawn|Components|CharacterMovement|SetMovementMode (Variables|/Script/Engine.Character|GetCharacterMovement _asbp_third_person_character_2) "MOVE_Walking" 0))
          (:else))))))

(event EventBeginPlay
  ;[0.15 0.15 0.15 0.5] 初始化
  (bind _asbp_third_person_character (Utilities|Casting|CastToBP_ThirdPersonCharacter (Components|GetOwner)))
  (Variables|Default|SetFollow%20Camera (Variables|/Game/RPG_Character/ThirdPerson/Blueprints/BP_ThirdPersonCharacter.BP_ThirdPersonCharacter_C|GetFollowCamera _asbp_third_person_character))
  (Variables|Default|SetBPC%20Attack%20System (Variables|/Game/RPG_Character/ThirdPerson/Blueprints/BP_ThirdPersonCharacter.BP_ThirdPersonCharacter_C|GetBPC_AttackSystem _asbp_third_person_character)))

(event Input|KeyboardEvents|DebugKeyH
  (params (Key :type Key%20Structure) (ActionValue :type Input%20Action%20Value%20Structure))
  ;[0.15 0.15 0.15 0.5] 拾取武器（利用球形追踪）
  (:Pressed
    (for _array_element (Variables|Default|GetWeaponSlots)
      (Development|PrintString (Utilities|String|ToString(Name) (.rowname (.item _array_element))) true true "(R=0.000000,G=0.660000,B=1.000000,A=1.000000)" 5.0))))

(fn AddWeapon
  (params (NewItem :type S%20Slots%20Structure%20%28by%20ref%29))
  (Utilities|Array|Add (Variables|Default|GetWeaponSlots) NewItem))