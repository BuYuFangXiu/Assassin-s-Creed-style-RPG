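; Boss AI actor that feeds its health state to its AI controller.
; Every Tick, after the parent logic, it casts its controller to BP_AIController_BOSS and copies current and max health from BPCPlayerStats into it.
; The construction script only calls the parent, and the BeginPlay and overlap events are inactive placeholders.
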(event `self.ReceiveTick`
  (params (DeltaSeconds :type "Float (single-precision)"))
  (bind _bpc_playerstats (`self.BPC_PlayerStats`))
  (`parent.ReceiveTick` DeltaSeconds)
  (bind _asbp_aicontroller_boss (cast `/Game/AI/BOSS/BP_AIController_BOSS` (`AIBlueprintHelperLibrary.GetAIController` self)))
  (set `/Game/AI/BOSS/BP_AIController_BOSS.Health` (`/Game/BluePrints/BPC_PlayerStats.Current Health` _bpc_playerstats) _asbp_aicontroller_boss)
  (set `/Game/AI/BOSS/BP_AIController_BOSS.Max Health` (`/Game/BluePrints/BPC_PlayerStats.Max Health` _bpc_playerstats) _asbp_aicontroller_boss))

(fn `UserConstructionScript`
  (`parent.UserConstructionScript`))