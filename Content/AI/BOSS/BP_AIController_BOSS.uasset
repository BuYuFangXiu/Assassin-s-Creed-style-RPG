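; AI controller for a boss enemy that runs the BT_AI_BOSS behavior tree on BeginPlay.
; ActivateBOSSCombat creates the boss health bar widget and adds it to the viewport; DeactivateBOSSCombat removes it and clears the reference.
; While the widget is valid, Tick sets its progress bar to Health divided by MaxHealth every frame.
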(event `self.ReceiveBeginPlay`
  ; 运行行为树
  (`self.RunBehaviorTree` "/Game/AI/BOSS/BT_AI_BOSS.BT_AI_BOSS"))

(event `Activate BOSS Combat`
  ; 将BOSS血量UI添加到玩家视口
  (bind _returnvalue (`|CreateWidget` "/Game/RPG_Character/UI/WB_BOSSHealthBar.WB_BOSSHealthBar_C"))
  (bind _output_get (set `self.BOSS Health Bar Widget` _returnvalue))
  (`UserWidget.AddToViewport` _output_get 0))

(event `Deactivate BOSS Combat`
  ; 将BOSS血量UI从玩家视口上移除
  (`Widget.RemoveFromParent` (`self.BOSS Health Bar Widget`))
  (set `self.BOSS Health Bar Widget` null))

(event `self.ReceiveTick`
  (params (DeltaSeconds :type "Float (single-precision)"))
  ; BOSS血量动态变化
  (bind _boss_health_bar_widget (`self.BOSS Health Bar Widget`)
    (:`then`
      (`ProgressBar.SetPercent` (`/Game/RPG_Character/UI/WB_BOSSHealthBar.HealthBar` _boss_health_bar_widget) (/ (`self.Health`) (`self.Max Health`))))
    (:`else`)))

(fn `UserConstructionScript`
  (`parent.UserConstructionScript`))