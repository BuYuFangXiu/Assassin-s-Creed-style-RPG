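; General AI controller that runs BT_AI and turns perception updates into blackboard data for chasing and investigating.
; Each update feeds both handlers: sight sets Target Actor and activates combat on boss controllers, while hearing sets Investigation Location and shows the pawn's investigation icon.
; Failed or non-sight stimuli clear the target and deactivate boss combat.
; Investigation Location is written for every stimulus, whatever its sense or success.
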(event `self.ReceiveBeginPlay`
  ; 执行行为树
  (`self.RunBehaviorTree` "/Game/AI/BT_AI.BT_AI"))

(event `self.AIPerception.OnTargetPerceptionUpdated`
  (params (Actor :type "Actor Object Reference") (Stimulus :type "AIStimulus Structure"))
  ; 检测并追逐/调查目标
  (`self. Sight Detection` Actor Stimulus)
  (`self.Hearing Detection` Actor Stimulus))

(fn ` Sight Detection`
  (params (Actor :type "Actor Object Reference") (Stimulus :type "AIStimulus Structure"))
  ; 检测并追逐目标
  (bind _returnvalue (`AIPerceptionSystem.GetSenseClassForStimulus` Stimulus))
  (if (== _returnvalue "/Script/AIModule.AISense_Sight")
    (if (`.bSuccessfullySensed` (break `AIStimulus` Stimulus))
      (`BlackboardComponent.SetValueAsObject` (`AIBlueprintHelperLibrary.GetBlackboard` null) "Target Actor" Actor)
      (bind _asbp_aicontroller_boss (cast `/Game/AI/BOSS/BP_AIController_BOSS` self))
      (`/Game/AI/BOSS/BP_AIController_BOSS.Activate BOSS Combat` _asbp_aicontroller_boss)
      (else
        (`BlackboardComponent.SetValueAsObject` (`AIBlueprintHelperLibrary.GetBlackboard` null) "Target Actor" null :!label _label)
        (bind _asbp_aicontroller_boss_2 (cast `/Game/AI/BOSS/BP_AIController_BOSS` self))
        (`/Game/AI/BOSS/BP_AIController_BOSS.Deactivate BOSS Combat` _asbp_aicontroller_boss_2)))
    (else
      (goto _label))))

(fn `Hearing Detection`
  (params (Actor :type "Actor Object Reference") (Stimulus :type "AIStimulus Structure"))
  (bind (_age _expirationage _strength _stimuluslocation _receiverlocation _tag _bsuccessfullysensed) (break `AIStimulus` Stimulus))
  ; 检测并监听位置
  (bind _returnvalue (`AIPerceptionSystem.GetSenseClassForStimulus` Stimulus))
  (if (== _returnvalue "/Script/AIModule.AISense_Hearing")
    (if _bsuccessfullysensed
      (`BlackboardComponent.SetValueAsVector` (`AIBlueprintHelperLibrary.GetBlackboard` null) "Investigation Location" _stimuluslocation)
      (bind _asbp_ai (cast `/Game/AI/BP_AI` (`self.K2_GetPawn`)))
      (`/Game/AI/BP_AI.Investigation Icon` _asbp_ai)
      (else
        (`BlackboardComponent.SetValueAsVector` (`AIBlueprintHelperLibrary.GetBlackboard` null) "Investigation Location" _stimuluslocation :!label _label)))
    (else
      (goto _label))))

(fn `UserConstructionScript`)