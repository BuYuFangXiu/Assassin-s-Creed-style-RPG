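; Enemy AI character with sword melee, health and stealth back-assassination by the player.
; Attack calls run a buffered three-montage combo, while timer-driven sphere traces deal damage to tagged actors.
; Damage cancels combos, plays random hit reactions and applies knockback; death ragdolls and notifies the player's quest component.
; An overlap reveals the assassination prompt, the takedown plays a paired victim montage before ragdolling, and widgets face the camera.
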(event `self.ReceiveBeginPlay`
  ; 初始化
  (bind _aswb_enemy_hud (cast `/Game/RPG_Character/UI/WB_EnemyHUD` (`WidgetComponent.GetWidget` (`self.Health Bar Widget`))))
  (set `self.HUD Widget` _aswb_enemy_hud))

(event `self.ReceiveTick`
  (params (DeltaSeconds :type "Float (single-precision)"))
  ; 可刺杀UI跟随人物视角的转动而转动
  (`SceneComponent.K2_SetWorldRotation` (`self.InvestigationIcon Widget`) (`KismetMathLibrary.FindLookAtRotation` (`SceneComponent.K2_GetComponentLocation` (`self.Assassinate Widget`)) (`SceneComponent.K2_GetComponentLocation` (`PlayerCameraManager.TransformComponent` (`GameplayStatics.GetPlayerCameraManager` 0)))) false false)
  (`SceneComponent.K2_SetWorldRotation` (`self.Assassinate Widget`) (`KismetMathLibrary.FindLookAtRotation` (`SceneComponent.K2_GetComponentLocation` (`self.Assassinate Widget`)) (`SceneComponent.K2_GetComponentLocation` (`PlayerCameraManager.TransformComponent` (`GameplayStatics.GetPlayerCameraManager` 0)))) false false)
  (`SceneComponent.K2_SetWorldRotation` (`self.Health Bar Widget`) (`KismetMathLibrary.FindLookAtRotation` (`SceneComponent.K2_GetComponentLocation` (`self.Assassinate Widget`)) (`SceneComponent.K2_GetComponentLocation` (`PlayerCameraManager.TransformComponent` (`GameplayStatics.GetPlayerCameraManager` 0)))) false false))

(event `Rogdoll`
  ; 布娃娃效果
  (`|ExecutionSequence`
    (:`then_0`
      (`KismetSystemLibrary.Delay` 2.5)
      (`PrimitiveComponent.SetSimulatePhysics` (`self.Mesh`) true)
      (bind _asbp_third_person_character (cast `/Game/RPG_Character/ThirdPerson/Blueprints/BP_ThirdPersonCharacter` (`GameplayStatics.GetPlayerCharacter` 0)))
      (set `/Game/RPG_Character/ThirdPerson/Blueprints/BP_ThirdPersonCharacter.IsAssassined` true _asbp_third_person_character))
    (:`then_1`
      (`KismetSystemLibrary.Delay` 1.6)
      (`GameplayStatics.PlaySoundAtLocation` "/Game/Audio/Grunt-Hits/Death1.Death1" (`self.K2_GetActorLocation`) (struct) 1.0 1.0 0.0 null null null null))))

(event `self. Assasination Radius.OnComponentBeginOverlap`
  (params (OverlappedComponent :type "PrimitiveComponent Object Reference") (OtherActor :type "Actor Object Reference") (OtherComp :type "PrimitiveComponent Object Reference") (OtherBodyIndex :type Integer) (bFromSweep :type Boolean) (SweepResult :type "HitResult Structure (by ref)"))
  ; 可刺杀的UI界面：接近敌人背后出现可刺杀标志
  (bind _asbp_third_person_character (cast `/Game/RPG_Character/ThirdPerson/Blueprints/BP_ThirdPersonCharacter` OtherActor))
  (if (not (`/Game/RPG_Character/ThirdPerson/Blueprints/BP_ThirdPersonCharacter.IsAssassined` _asbp_third_person_character))
    (`SceneComponent.SetVisibility` (`self.Assassinate Widget`) true false)))

(event `self. Assasination Radius.OnComponentEndOverlap`
  (params (OverlappedComponent :type "PrimitiveComponent Object Reference") (OtherActor :type "Actor Object Reference") (OtherComp :type "PrimitiveComponent Object Reference") (OtherBodyIndex :type Integer))
  ; 可刺杀的UI界面：离开敌人背后刺杀标志消失
  (cast `/Game/RPG_Character/ThirdPerson/Blueprints/BP_ThirdPersonCharacter` OtherActor)
  (`SceneComponent.SetVisibility` (`self.Assassinate Widget`) false false))

(event `self.ReceiveAnyDamage`
  (params (Damage :type "Float (single-precision)") (DamageType :type "DamageType Object Reference") (InstigatedBy :type "Controller Object Reference") (DamageCauser :type "Actor Object Reference"))
  ; 受击时播放受击动画并玩家击退、以及攻击玩家后扣除生命值至死亡
  (`self.Stop Combo`)
  (`self.PlayAnimMontage` (`|GetArrayItem` (`self.HitAnims`) (`KismetMathLibrary.RandomIntegerInRange` 0 (- (`KismetArrayLibrary.Array_Length` (`self.HitAnims`)) 1))))
  (bind _asbp_third_person_character (cast `/Game/RPG_Character/ThirdPerson/Blueprints/BP_ThirdPersonCharacter` (`GameplayStatics.GetPlayerCharacter` 0)))
  (`self.LaunchCharacter` (* (`KismetMathLibrary.GetForwardVector` (`self.K2_GetActorRotation` _asbp_third_person_character)) 700.0))
  (`GameplayStatics.PlaySoundAtLocation` "/Game/Audio/Grunt-Hits/Grunt.Grunt" (`self.K2_GetActorLocation`) (struct) 1.0 (`KismetMathLibrary.RandomFloatInRange` 1.0 3.0) 0.0 "/Game/Audio/SA_Character.SA_Character" null null null)
  (bind _is_player_death_ (`/Game/BluePrints/BPC_PlayerStats.Decrease Health` (`self.BPC_PlayerStats`) Damage))
  (if _is_player_death_
    ; 测试死亡（仅用于测试）
    (`PrimitiveComponent.SetCollisionObjectType` (`self.Mesh`) "ECC_PhysicsBody")
    (`self.Rogdoll`)
    (`|ExecutionSequence`
      (:`then_0`
        (`PrimitiveComponent.SetSimulatePhysics` (`self.Mesh`) true)
        (bind _asbp_third_person_character_2 (cast `/Game/RPG_Character/ThirdPerson/Blueprints/BP_ThirdPersonCharacter` (`GameplayStatics.GetPlayerCharacter` 0)))
        (set `/Game/RPG_Character/ThirdPerson/Blueprints/BP_ThirdPersonCharacter.IsAssassined` true _asbp_third_person_character_2))
      (:`then_1`
        (`GameplayStatics.PlaySoundAtLocation` "/Game/Audio/Grunt-Hits/Death1.Death1" (`self.K2_GetActorLocation`) (struct) 1.0 1.0 0.0 null null null null)
        (`SceneComponent.SetVisibility` (`self.Health Bar Widget`) false false)
        (`SceneComponent.SetVisibility` (`self.Assassinate Widget`) false false)
        (`CharacterMovementComponent.SetMovementMode` (`self.CharacterMovement`) "MOVE_None" 0)
        (bind _asbp_third_person_character_3 (cast `/Game/RPG_Character/ThirdPerson/Blueprints/BP_ThirdPersonCharacter` (`GameplayStatics.GetPlayerCharacter` 0)))
        (`/Game/Quest_System/BPC_Quest.Eliminate Enemy` (`/Game/RPG_Character/ThirdPerson/Blueprints/BP_ThirdPersonCharacter.BPC_Quest` _asbp_third_person_character_3) self)))))

(event `Attack 1`
  ; 连击系统
  ;; 攻击1
  (`/Engine/EditorBlueprintResources/StandardMacros.DoOnce` false :!label _label
    (:`Completed`
      (`KismetSystemLibrary.Delay` 0.1)
      (`|PlayMontage` (`self.Mesh`) "/Game/RPG_Character/Animations/SwordAttacks/Attack1_Montage.Attack1_Montage" (`self.Attack Animation Rate`)
        (:`then`
          (set `self.Attack Index` 1)
          (goto _label :!via `Reset`))))))

(event `Sword Attack Combo Call From BT`
  ; 连击系统
  ;; 攻击输入
  (if (`self.Can Attack?`)
    (`self.SwordAttack`)))

(event `Attack 2`
  ; 连击系统
  ;; 攻击2
  (`/Engine/EditorBlueprintResources/StandardMacros.DoOnce` false :!label _label_2
    (:`Completed`
      (`KismetSystemLibrary.Delay` 0.1)
      (`|PlayMontage` (`self.Mesh`) "/Game/RPG_Character/Animations/SwordAttacks/Attack2_Montage.Attack2_Montage" (`self.Attack Animation Rate`)
        (:`then`
          (set `self.Attack Index` 2)
          (goto _label_2 :!via `Reset`))))))

(event `SwordAttack`
  ; 连击系统
  ;; 剑攻击
  (if (`self.Is Attacking?`)
    (set `self.Save Attack?` true)
    (else
      (set `self.Is Attacking?` true)
      (switch `int` (`self.Attack Index`) :!label _label_3
        (:`0`
          (`self.Attack 1`))
        (:`1`
          (`self.Attack 2`))
        (:`2`
          (`self.Attack 4`))))))

(event `Sword Attack Combo`
  ; 连击系统
  ;; 连击功能
  (if (`self.Save Attack?`)
    (set `self.Save Attack?` false)
    (goto _label_3)
    (else
      (`self.Stop Combo`))))

(event `Attack 3`
  ; 连击系统
  ;; 攻击3（未使用）
  (`/Engine/EditorBlueprintResources/StandardMacros.DoOnce` false :!label _label_4
    (:`Completed`
      (`KismetSystemLibrary.Delay` 0.1)
      (`|PlayMontage` (`self.Mesh`) "/Game/RPG_Character/Animations/SwordAttacks/Kick_Montage.Kick_Montage" 1.0 (`self.Attack Animation Rate`)
        (:`then`
          (set `self.Attack Index` 3)
          (goto _label_4 :!via `Reset`))))))

(event `Stop Combo`
  ; 连击系统
  ;; 停止攻击和连击
  (set `self.Is Attacking?` false)
  (set `self.Attack Index` 0))

(event `Attack 4`
  ; 连击系统
  ;; 攻击4
  (`/Engine/EditorBlueprintResources/StandardMacros.DoOnce` false :!label _label_5
    (:`Completed`
      (`KismetSystemLibrary.Delay` 0.1)
      (`|PlayMontage` (`self.Mesh`) "/Game/RPG_Character/Animations/SwordAttacks/Attack3_Montage.Attack3_Montage" (`self.Attack Animation Rate`)
        (:`then`
          (set `self.Attack Index` 0)
          (goto _label_5 :!via `Reset`))))))

(event `Start Sword Trace`
  ; 剑的伤害追踪
  (bind _returnvalue (`KismetSystemLibrary.K2_SetTimerDelegate` (delegate `Sword Trace Loop`) 0.001 true))
  (set `self.SwordTraceLoop` _returnvalue))

(event `Sword Trace Loop`
  ; 剑的伤害追踪
  (bind (_outhit _returnvalue) (`KismetSystemLibrary.SphereTraceSingle` :`Start` (`SceneComponent.K2_GetComponentLocation` (`self.Sword Top Point`)) :`End` (`SceneComponent.K2_GetComponentLocation` (`self.Sword Bottom Point`)) :`Radius` 5.0 :`TraceChannel` "TraceTypeQuery1" :`DrawDebugType` "ForDuration" :`DrawTime` 0.2))
  (if _returnvalue
    (bind (_bblockinghit _binitialoverlap _time _distance _location _impactpoint _normal _impactnormal _physmat _hitactor) (`GameplayStatics.BreakHitResult` _outhit))
    (if (`self.ActorHasTag` _hitactor "Damegeable")
      (`/Engine/EditorBlueprintResources/StandardMacros.DoOnce` false :!label _label_6
        (:`Completed`
          (`GameplayStatics.ApplyDamage` _hitactor (`self.Sword Damage`))
          (`GameplayStatics.PlayWorldCameraShake` "/Game/BluePrints/BP_CameraShake_SwordHit.BP_CameraShake_SwordHit_C" _location 0.0 2000.0)
          (`self.Play Sword Hit Sounds`)
          (`GameplayStatics.SpawnEmitterAtLocation` "/Game/FXs/Particles/Blood/P_Blood_Splat_Cone.P_Blood_Splat_Cone" _location (`KismetMathLibrary.MakeRotFromXY` _normal _normal) (0.4 0.4 0.4) true "AutoRelease")
          (`KismetSystemLibrary.Delay` 0.3)
          (goto _label_6 :!via `Reset`))))))

(event `Stop Sword Trace`
  ; 剑的伤害追踪
  ;; 中断攻击连击
  (`KismetSystemLibrary.K2_ClearAndInvalidateTimerHandle` (`self.SwordTraceLoop`)))

(event `Sphere Trace`
  (bind _returnvalue (`SceneComponent.K2_GetComponentLocation` (`self.Sphere Trace Pos`)))
  ; 通用伤害追踪（踢击以及更多其他）
  (bind (_outhit _returnvalue_2) (`KismetSystemLibrary.SphereTraceSingle` :`Start` _returnvalue :`End` _returnvalue :`Radius` 35.0 :`TraceChannel` "TraceTypeQuery1" :`DrawDebugType` "ForDuration" :`DrawTime` 0.2))
  (if _returnvalue_2
    (bind (_bblockinghit _binitialoverlap _time _distance _location _impactpoint _normal _impactnormal _physmat _hitactor) (`GameplayStatics.BreakHitResult` _outhit))
    (if (`self.ActorHasTag` _hitactor "Damegeable")
      (`GameplayStatics.ApplyDamage` _hitactor (`self.Kich Damage`))
      (`GameplayStatics.PlayWorldCameraShake` "/Game/BluePrints/BP_CameraShake_SwordHit.BP_CameraShake_SwordHit_C" _location 0.0 2000.0)
      (`GameplayStatics.SpawnEmitterAtLocation` "/Game/FXs/Particles/Blood/P_Blood_Splat_Cone.P_Blood_Splat_Cone" _location (`KismetMathLibrary.MakeRotFromXY` _normal _normal) (0.4 0.4 0.4) true "AutoRelease"))))

(event `Play Sword Hit Sounds`
  ; 播放剑击打声音
  (`GameplayStatics.PlaySoundAtLocation` "/Game/Audio/Sword_Hit/MS_SwordHit.MS_SwordHit" (`self.K2_GetActorLocation` (`self.GetOwner`)) (struct) 1.0 1.0 0.0 null null null null))

(event `Investigation Icon`
  (bind _investigationicon_widget (`self.InvestigationIcon Widget`))
  ; 警惕图标的可见/不可见
  (`/Engine/EditorBlueprintResources/StandardMacros.FlipFlop`
    (:`A`
      (`SceneComponent.SetVisibility` _investigationicon_widget true false))
    (:`B`
      (`SceneComponent.SetVisibility` _investigationicon_widget false false))))

(fn `Attack`
  (returns (`Animation Duration` :type "Float (double-precision)"))
  (`self.Sword Attack Combo Call From BT`)
  (return 0.4))

(fn `Stealth Back Assassination`
  (returns (`REF Location` :type "Vector Structure") (`Assassin Rotation` :type "Rotator Structure"))
  (`self.PlayAnimMontage` "/Game/RPG_Character/Animations/Assassinations/Paired_Knife_Stealth_KidneyAndNeck_Vic1_Montage.Paired_Knife_Stealth_KidneyAndNeck_Vic1_Montage")
  (`self.Rogdoll`)
  (`SceneComponent.SetVisibility` (`self.Assassinate Widget`) false false)
  (`SceneComponent.SetVisibility` (`self.Health Bar Widget`) false false)
  (`CharacterMovementComponent.SetMovementMode` (`self.CharacterMovement`) "MOVE_None" 0)
  (return (`SceneComponent.K2_GetComponentLocation` (`self.Assassin REF(可视性已关闭)`)) (`self.K2_GetActorRotation`)))

(fn `UserConstructionScript`)