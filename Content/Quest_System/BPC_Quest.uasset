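; Quest component that tracks one active quest's eliminate-enemy and open-chest objectives and drives the quest HUD.
; It creates WB_QuestHUD shortly after BeginPlay, hidden until the active quest text is set, and fills its objective list on request.
; Enemy kills shrink a working target array, while chest openings match the objective's chest.
; Each finished objective updates the HUD and a counter, which clears the quest and plays the completion animation when all are done.
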(event `self.ReceiveBeginPlay`
  (`KismetSystemLibrary.Delay` 0.2)
  (bind _returnvalue (`|CreateWidget` "/Game/Quest_System/WB_QuestHUD.WB_QuestHUD_C"))
  (bind _output_get (set `self.Quest HUD WIdget` _returnvalue))
  (`UserWidget.AddToViewport` _output_get 0)
  (`/Game/Quest_System/WB_QuestHUD.Hide Quest Panel` (`self.Quest HUD WIdget`)))

(event `Set Active Quest Text`
  (`TextBlock.SetText` (`/Game/Quest_System/WB_QuestHUD.ActiveQuestText` (`self.Quest HUD WIdget`)) (`KismetTextLibrary.Conv_StringToText` (`.Name_2_95045E9440CD342237B196A27F5EB2E6` (break `/Game/Quest_System/S_Quest` (`self.Active Quest`)))))
  (`/Game/Quest_System/WB_QuestHUD.Shou Quest Panel` (`self.Quest HUD WIdget`)))

(event `Set Objectives`
  (bind (_active_quest_name _active_quest_description _active_quest_secundary _active_quest_completed _active_quest_objevtives) (break `/Game/Quest_System/S_Quest` (`self.Active Quest`)))
  (`/Game/Quest_System/WB_QuestHUD.Fill Objective` (`self.Quest HUD WIdget`) _active_quest_objevtives))

(event `Eliminate Enemy`
  (params (`Eliminated Enemy` :type "Actor Object Reference"))
  (bind (_active_quest_name _active_quest_description _active_quest_secundary _active_quest_completed _active_quest_objevtives) (break `/Game/Quest_System/S_Quest` (`self.Active Quest`)))
  (bind _returnvalue (`KismetArrayLibrary.Array_Length` (`self.Enemy Actors Array`)))
  (for _array_element _active_quest_objevtives
    (bind (_nameaim _completed _actorstoeliminate _chesttoopen _iseliminateenemyobjective _ischestobjetive) (break `/Game/Quest_System/S_QuestObjective` _array_element))
    (if (and (not _completed) _iseliminateenemyobjective)
      (if (not (!= (`KismetArrayLibrary.Array_Length` (`self.Enemy Actors Array`)) 0))
        (bind _output_get (set `self.Enemy Actors Array` _actorstoeliminate)))
      (`KismetArrayLibrary.Array_RemoveItem` _output_get `Eliminated Enemy`)
      (`|VariableSetRef` _array_element (make `/Game/Quest_System/S_QuestObjective` _nameaim true (`self.Enemy Actors Array`) _chesttoopen _iseliminateenemyobjective _ischestobjetive))
      (`KismetSystemLibrary.PrintString` (`KismetStringLibrary.Conv_IntToString` _returnvalue))
      (if (== _returnvalue 0)
        (`|VariableSetRef` _array_element (make `/Game/Quest_System/S_QuestObjective` _nameaim true _ _chesttoopen _iseliminateenemyobjective _ischestobjetive))
        (`/Game/Quest_System/WB_QuestHUD.Complete Objective` (`self.Quest HUD WIdget`) _array_element)
        (`self.Objective Completed`)
        (`KismetSystemLibrary.PrintString` "Complete")))))

(event `Open Chest`
  (params (Chest :type "Actor Object Reference"))
  (bind (_active_quest_name _active_quest_description _active_quest_secundary _active_quest_completed _active_quest_objevtives) (break `/Game/Quest_System/S_Quest` (`self.Active Quest`)))
  (for _array_element _active_quest_objevtives
    (bind (_nameaim _completed _actorstoeliminate _chesttoopen _iseliminateenemyobjective _ischestobjetive) (break `/Game/Quest_System/S_QuestObjective` _array_element))
    (if (and _ischestobjetive (== _chesttoopen Chest))
      (`|VariableSetRef` _array_element (make `/Game/Quest_System/S_QuestObjective` _nameaim false _actorstoeliminate null _iseliminateenemyobjective _ischestobjetive))
      (`/Game/Quest_System/WB_QuestHUD.Complete Objective` (`self.Quest HUD WIdget`) _array_element)
      (`self.Objective Completed`)
      (`KismetSystemLibrary.PrintString` "Complete"))))

(event `Objective Completed`
  (bind (_active_quest_name _active_quest_description _active_quest_secundary _active_quest_completed _active_quest_objevtives) (break `/Game/Quest_System/S_Quest` (`self.Active Quest`)))
  (`/Engine/EditorBlueprintResources/StandardMacros.IncrementInt` (`self.ObjectiveCompleted`)
    (:`  `
      (if (>= (`self.ObjectiveCompleted`) (`KismetArrayLibrary.Array_Length` _active_quest_objevtives))
        (`KismetSystemLibrary.PrintString` "Quest Completed")
        (set `self.Active Quest` (struct))
        (set `self.ObjectiveCompleted` 0)
        (`/Game/Quest_System/WB_QuestHUD.Play Quest Completed Animation` (`self.Quest HUD WIdget`))))))