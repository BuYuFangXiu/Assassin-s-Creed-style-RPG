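; BP_QuestGiver is an interactable quest giver that plays a dialogue, then offers its quests.
; A trigger radius toggles a camera-facing prompt, reused from an assassination indicator and shown only if the character's IsAssassined is false.
; Interact opens the dialogue widget, steps through the Dialogue array, then fills WB_QuestGiver from the Quest array.
; Interacting again closes the quest window and restores game-only input.
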(event `self.ReceiveTick`
  (params (DeltaSeconds :type "Float (single-precision)"))
  (bind _interact_widget (`self.Interact Widget`))
  ; 可刺杀UI跟随人物视角的转动而转动
  (`SceneComponent.K2_SetWorldRotation` _interact_widget (`KismetMathLibrary.FindLookAtRotation` (`SceneComponent.K2_GetComponentLocation` _interact_widget) (`SceneComponent.K2_GetComponentLocation` (`PlayerCameraManager.TransformComponent` (`GameplayStatics.GetPlayerCameraManager` 0)))) false false))

(event `self.Trigger Radius.OnComponentBeginOverlap`
  (params (OverlappedComponent :type "PrimitiveComponent Object Reference") (OtherActor :type "Actor Object Reference") (OtherComp :type "PrimitiveComponent Object Reference") (OtherBodyIndex :type Integer) (bFromSweep :type Boolean) (SweepResult :type "HitResult Structure (by ref)"))
  ; 可刺杀的UI界面：接近敌人背后出现可刺杀标志（在这里改为了可对话功能）
  (bind _asbp_third_person_character (cast `/Game/RPG_Character/ThirdPerson/Blueprints/BP_ThirdPersonCharacter` OtherActor))
  (if (not (`/Game/RPG_Character/ThirdPerson/Blueprints/BP_ThirdPersonCharacter.IsAssassined` _asbp_third_person_character))
    (`SceneComponent.SetVisibility` (`self.Interact Widget`) true false)))

(event `self.Trigger Radius.OnComponentEndOverlap`
  (params (OverlappedComponent :type "PrimitiveComponent Object Reference") (OtherActor :type "Actor Object Reference") (OtherComp :type "PrimitiveComponent Object Reference") (OtherBodyIndex :type Integer))
  ; 可刺杀的UI界面：离开敌人背后刺杀标志消失（在这里改为了可对话功能）
  (cast `/Game/RPG_Character/ThirdPerson/Blueprints/BP_ThirdPersonCharacter` OtherActor)
  (`SceneComponent.SetVisibility` (`self.Interact Widget`) false false))

(event `Open Quests Widget`
  ; 对话窗口和任务
  (bind _returnvalue (`|GenericCreateObject` "/Game/Quest_System/WB_QuestGiver.WB_QuestGiver_C"))
  (bind _output_get (set `self.Widget` _returnvalue))
  (`UserWidget.AddToViewport` _output_get 0)
  (set `self.Widget Active` true)
  (set `/Game/Quest_System/WB_QuestGiver.Quest Giver BP` self (`self.Widget`))
  (for _array_element (`self.Quest`)
    (`/Game/Quest_System/WB_QuestGiver.Add Quest` (`self.Widget`) _array_element)))

(event `Close Quests Widget`
  (bind _returnvalue (`GameplayStatics.GetPlayerController` 0))
  ; 对话窗口和任务
  (`Widget.RemoveFromParent` (`self.Widget`) :!label _label)
  (set `self.Widget` null)
  (set `PlayerController.bShowMouseCursor` false _returnvalue)
  (`WidgetBlueprintLibrary.SetInputMode_GameOnly` _returnvalue)
  (set `self.Widget Active` false))

(event `/Game/Quest_System/BPI_QuestGiver.Interact`
  (bind _returnvalue (`GameplayStatics.GetPlayerController` 0))
  ; 对话窗口和任务
  (if (not (`self.Widget Active`))
    (if (not (`self.IsDialogueOpened?`))
      (bind _returnvalue_2 (`|GenericCreateObject` "/Game/Quest_System/WB_QuestGieverDialogue.WB_QuestGieverDialogue_C"))
      (bind _output_get (set `self.Dialogue Widget` _returnvalue_2))
      (`UserWidget.AddToViewport` _output_get 0)
      (set `self.IsDialogueOpened?` true)
      (set `PlayerController.bShowMouseCursor` true _returnvalue)
      (`WidgetBlueprintLibrary.SetInputMode_GameAndUIEx` _returnvalue (`self.Widget`))
      (else
        (`TextBlock.SetText` (`/Game/Quest_System/WB_QuestGieverDialogue.DialogueText` (`self.Dialogue Widget`)) (`KismetTextLibrary.Conv_StringToText` (`|GetArrayItem` (`self.Dialogue`) (`self.DialogueIndex`))))
        (`/Engine/EditorBlueprintResources/StandardMacros.IncrementInt` (`self.DialogueIndex`)
          (:`  `
            (if (> (`self.DialogueIndex`) (`KismetArrayLibrary.Array_Length` (`self.Dialogue`)))
              (`Widget.RemoveFromParent` (`self.Dialogue Widget`))
              (set `self.Dialogue Widget` null)
              (set `self.DialogueIndex` 0)
              (set `self.IsDialogueOpened?` false)
              (`self.Open Quests Widget`))))))
    (else
      (goto _label))))

(fn `UserConstructionScript`)